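; BP_CharacterBase is the base character Blueprint that handles switching between a main and a sub weapon.
; Two server-named events show one weapon actor, hide the other with SetActorHiddenInGame, and call ServerOnWeaponEquipped on the shown weapon, passing the character.
; An unconnected authority-checked visibility branch and calls to ServerMainWeapon and ServerSubWeapon never run, and the construction script is empty.
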(event `Server_MainWeapon`
  (bind _mainweapon (`self.MainWeapon`))
  (`self.SetActorHiddenInGame` _mainweapon false)
  (`self.SetActorHiddenInGame` (`self.SubWeapon`) true)
  (`FPSWeaponBase.Server_OnWeaponEquipped` _mainweapon self))

(event `Server_SubWeapon`
  (bind _subweapon (`self.SubWeapon`))
  (`self.SetActorHiddenInGame` (`self.MainWeapon`) true)
  (`self.SetActorHiddenInGame` _subweapon false)
  (`FPSWeaponBase.Server_OnWeaponEquipped` _subweapon self))

(fn `UserConstructionScript`)