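; BP_ProjectileBase is, by name, the base projectile Blueprint for the FPS weapons, though it holds only debug and test movement logic.
; Tick prints the owner's display name every frame.
; Server_Move accumulates DeltaTime into Time and offsets the actor's Z by its cosine for a vertical bob, with no forward travel.
; Nothing in this graph calls Server_Move, and there is no overlap or hit handling.
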(event `self.ReceiveTick`
  (params (DeltaSeconds :type "Float (single-precision)"))
  (`KismetSystemLibrary.PrintString` (`KismetSystemLibrary.GetDisplayName` (`self.GetOwner`))))

(event `Server_Move`
  (params (DeltaTime :type "Float (double-precision)"))
  (bind (_returnvalue_x _returnvalue_y _returnvalue_z) (`KismetMathLibrary.BreakVector` (`self.K2_GetActorLocation`)))
  (set `self.Time` (+ DeltaTime (`self.Time`)))
  (`self.K2_SetActorLocation` (`KismetMathLibrary.MakeVector` _returnvalue_x _returnvalue_y (+ _returnvalue_z (* (`KismetMathLibrary.Cos` (`self.Time`)) 1.0)))))

(fn `UserConstructionScript`)