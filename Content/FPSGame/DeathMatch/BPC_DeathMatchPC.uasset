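; DeathMatch player controller that shows a debug HUD of the match's player states.
; On BeginPlay, the server waits briefly, collects the DeathMatch player states from the GameState's PlayerArray once, then calls a client event to create the HUD widget.
; That event also starts a looping one-second timer that passes the stored array to the widget to refresh it.
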(event `self.ReceiveBeginPlay`
  (`/Engine/EditorBlueprintResources/ActorMacros.Switch Has Authority`
    (:`Authority`
      (`KismetSystemLibrary.Delay` 1.0)
      (for _array_element (`GameStateBase.PlayerArray` (`GameplayStatics.GetGameState`))
        (bind _asdeath_match_player_state (cast `DeathMatchPlayerState` _array_element))
        (`KismetArrayLibrary.Array_Add` (`self.PS`) _asdeath_match_player_state))
      (`self.Client_SetupDebugWidget`))))

(event `Client_SetupDebugWidget`
  (bind _returnvalue (`|CreateWidget` "/Game/FPSGame/UI/Debug/WBP_DebugHUD.WBP_DebugHUD_C"))
  (bind _output_get (set `self.DebugHUD` _returnvalue))
  (`UserWidget.AddToViewport` _output_get 0)
  (`KismetSystemLibrary.K2_SetTimerDelegate` (delegate `CustomTick`) 1.0 true))

(event `CustomTick`
  (`self.Client_UpdateDebugUI`))

(event `Client_UpdateDebugUI`
  (`/Game/FPSGame/UI/Debug/WBP_DebugHUD.UpdateUserDebug` (`self.DebugHUD`) (`self.PS`)))

(fn `UserConstructionScript`)